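; BP_SpeedPowerup is a powerup that temporarily changes the walk speed of the first player's pawn.
; On activation it caches the character movement component's current max speed and sets MaxWalkSpeed to that value times SpeedMultiplier.
; On expiry it writes the cached speed back to MaxWalkSpeed.
; ApplyPowerup is empty, and the file contains no timing logic of its own.
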(event EventOnActivated
  (bind _returnvalue (Game|Player|GetPlayerPawn 0))
  (bind _returnvalue_2 (Actor|GetComponentbyClass _returnvalue "/Script/Engine.CharacterMovementComponent"))
  (bind _output_get (Variables|Default|SetOriginalMaxSpeed (Class|MovementComponent|GetMaxSpeed _returnvalue_2)))
  (Variables|/Script/Engine.CharacterMovementComponent|SetMaxWalkSpeed _returnvalue_2 (* _output_get (Variables|Default|GetSpeedMultiplier))))

(event EventOnExpired
  (Variables|/Script/Engine.CharacterMovementComponent|SetMaxWalkSpeed (Actor|GetComponentbyClass (Game|Player|GetPlayerPawn 0) "/Script/Engine.CharacterMovementComponent") (Variables|Default|GetOriginalMaxSpeed)))

(event EventApplyPowerup)

(fn ConstructionScript)