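; BP_HordeGameMode is the horde game mode that spawns AI bots and awards score for kills.
; Its OnActorKilled event adds fixed points to the killer's CoopPlayerState when a non-player pawn dies, then prints the score.
; SpawnBot runs an EQS location query, whose callback draws debug spheres and randomly spawns BP_SmartAI or, more often, BP_Tracker, both given BT_SmartAI.
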(event Custom|OnQueryFinished
  (params (QueryInstance :type Env%20Query%20Instance%20Blueprint%20Wrapper%20Object%20Reference) (QueryStatus :type EEnvQueryStatus%20Enum :default "Processing"))
  ;[1 1 1] Spawn bot
  (switch Utilities|FlowControl|Switch|SwitchonEEnvQueryStatus QueryStatus
    (:Success
      (for _array_element (Class|EnvQueryInstanceBlueprintWrapper|GetResultsasLocations QueryInstance)
        (Rendering|Debug|DrawDebugSphere _array_element 5e+01 12 "(R=1.000000,G=0.000000,B=0.964583,A=1.000000)" 2.0 2.0)
        (AI|SpawnAIFromClass (select (<= (Math|Random|RandomFloatinRange 0.0 1e+02) 4e+01) "/Game/AdvancedAI/BP_SmartAI.BP_SmartAI_C" "/Game/AI/Tracker/BP_Tracker.BP_Tracker_C") "/Game/AdvancedAI/BT_SmartAI.BT_SmartAI" _array_element "0, 0, 0" false)))))

(event Custom|On%20Actor%20Killed
  (params (Victim :type Actor%20Object%20Reference) (Killer :type Actor%20Object%20Reference) (KillerController :type Controller%20Object%20Reference))
  ;[1 1 1] When a player is killed, health component triggers game mode to throw an event that catches from gm itself, to increase the score and report it
  (bind _aspawn (Utilities|Casting|CastToPawn Victim))
  (if (not (Pawn|IsPlayerControlled _aspawn))
    (Utilities|IsValid KillerController
      (:Is%20Valid
        (bind _playerstate (Variables|/Script/Engine.Pawn|GetPlayerState (Pawn|GetControlledPawn KillerController))
          (:then
            (bind _ascoop_player_state (Utilities|Casting|CastToCoopPlayerState _playerstate))
            (Class|CoopPlayerState|AddScore _ascoop_player_state 1e+01)
            (Development|PrintString (Utilities|String|Append "Score: " (Utilities|String|ToString(Float) (Variables|/Script/Engine.PlayerState|GetScore _ascoop_player_state)))))
          (:else))))))

(event EventBeginPlay
  ;[1 1 1] When a player is killed, health component triggers game mode to throw an event that catches from gm itself, to increase the score and report it
  (EventDispatchers|BindEventtoOnActorKilled (delegate Custom|On%20Actor%20Killed)))

(event EventTick
  (params (DeltaSeconds :type Float%20%28single-precision%29))
  ;[1 1 1] Spawn bot
)

(event EventSpawnBot
  ;[1 1 1] Spawn bot
  (bind _returnvalue (AI|EQS|RunEQSQuery "/Game/AI/Horde/EQS_FindSpawnLocation.EQS_FindSpawnLocation" self "RandomBest25Pct"))
  (EventDispatchers|BindEventtoOnQueryFinishedEvent _returnvalue (delegate Custom|OnQueryFinished)))

(fn ConstructionScript)