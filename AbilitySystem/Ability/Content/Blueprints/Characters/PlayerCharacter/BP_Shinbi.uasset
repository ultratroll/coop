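; BP_Shinbi is a player character Blueprint for Shinbi, with a sword melee attack driven by the Gameplay Ability System.
; BeginPlay acquires the GA_Melee ability and binds the sword capsule's begin-overlap event.
; MeleeAttack tries to activate GA_Melee by class through the ability system component.
; Sword overlaps with another ASCharacter only print a debug "Attack" string, with no damage applied here.
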(event Custom|MeleeAttack
  (Abilities|TryActivateAbilitybyClass (Variables|Default|GetAbilitySystemComp) "/Game/Blueprints/Characters/PlayerCharacter/Abilities/Melee/GA_Melee.GA_Melee_C" true))

(event Custom|Sword%20Overlap
  (params (OverlappedComponent :type Primitive%20Component%20Object%20Reference) (OtherActor :type Actor%20Object%20Reference) (OtherComp :type Primitive%20Component%20Object%20Reference) (OtherBodyIndex :type Integer) (bFromSweep :type Boolean) (SweepResult :type Hit%20Result%20Structure%20%28by%20ref%29))
  (bind _asascharacter (Utilities|Casting|CastToASCharacter OtherActor))
  (Utilities|IsValid _asascharacter
    (:Is%20Valid
      (if (!= _asascharacter self)
        (Development|PrintString "Attack")))))

(event EventBeginPlay
  (Class|ASCharacter|AcquireAbility "/Game/Blueprints/Characters/PlayerCharacter/Abilities/Melee/GA_Melee.GA_Melee_C")
  (Collision|BindEventtoOnComponentBeginOverlap (Variables|Default|GetSwordCapsule) (delegate Custom|Sword%20Overlap)))

(fn ConstructionScript)